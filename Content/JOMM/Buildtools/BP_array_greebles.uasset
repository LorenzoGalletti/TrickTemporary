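; BP_array_greebles is a level-building tool that scatters random greeble meshes in a 3D grid.
; The construction script creates one static HISM component per listed mesh, so the array previews live in the editor.
; Nested X, Z and Y loops add each instance to a randomly picked component, where empty list entries leave gaps.
; Rotation and spacing get unseeded random variation, with spacing jitter multiplied by grid index.
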(event Custom|Constructor
  ;[1 1 1] creates list of hieracheal meshes to use for random pattern
  (Utilities|Array|Clear (Variables|Default|GetHISMC%20list))
  (for _array_element (Variables|TOOLOPTIONS|GetStatic%20mesh%20list)
    (bind _returnvalue (AddComponent|AddHierarchicalInstancedStaticMeshComponent false))
    (Rendering|SetCastShadow _returnvalue (Variables|TOOLOPTIONS|Getcast%20shadows))
    (Transformation|SetMobility _returnvalue "Static")
    (Components|StaticMesh|SetStaticMesh _returnvalue _array_element)
    (Utilities|Array|AddUnique (Variables|Default|GetHISMC%20list) _returnvalue))
  (CallFunction|BuildXandY))

(event Custom|build%20x%20and%20y
  (bind (_x_spacing _y_spacing _z_spacing) (CallFunction|RandomiseXYZSpacing))
  ;[1 1 1] X and Z repeats (X handled as the 0 row of Z anyway)
  (for _index (range 0 (Variables|TOOLOPTIONS|GetX%20Repeats))
    (for _index_2 (range 0 (Variables|TOOLOPTIONS|GetZ%20repeats))
      (bind _output (CallFunction|Randomize))
      (Components|InstancedStaticMesh|AddInstance _output (Math|Transform|MakeTransform (Math|Vector|MakeVector (* _index _x_spacing) 0.0 (* _index_2 _z_spacing)) (CallFunction|RandomiseRotation) "1,1,1"))
      ;[1 1 1] Y repeats
      (for _index_3 (range 1 (Variables|TOOLOPTIONS|GetY%20Repeats))
        (bind _output_2 (CallFunction|Randomize))
        (Components|InstancedStaticMesh|AddInstance _output_2 (Math|Transform|MakeTransform (Math|Vector|MakeVector (* _index _x_spacing) (* _index_3 (.y%20spacing (CallFunction|RandomiseXYZSpacing))) (* _index_2 _z_spacing)) (CallFunction|RandomiseRotation) "1,1,1"))))))

(fn ConstructionScript
  ;[0 1 0] array Greebles:  Mark Seddon:  JOMM (Just One More Minute)
  (CallFunction|Constructor) ; Running this from here ensures you can see everything in realtime in editor and preserves navmesh update in game time
)

(fn Randomize
  (bind _hismc_list (Variables|Default|GetHISMC%20list))
  ;[1 1 1] picks a random greeble from the list created in the editor details.  Can also include random gaps by adding an empty into the list
  (return (Utilities|Array|Get(acopy) _hismc_list (Math|Random|RandomIntegerinRange 0 (Utilities|Array|LastIndex _hismc_list)))))

(fn RandomiseRotation
  (bind _rotation_variance (Variables|TOOLOPTIONS|GetRotation%20variance))
  ;[1 1 1] Random rotation for each greeble based on the parameters you set in the editor
  (return (Math|Rotator|MakeRotator (Math|Random|RandomFloatinRange (- 0.0 (.roll _rotation_variance)) (.roll _rotation_variance)) (Math|Random|RandomFloatinRange (- 0.0 (.pitch _rotation_variance)) (.pitch _rotation_variance)) (Math|Random|RandomFloatinRange (- 0.0 (.yaw _rotation_variance)) (.yaw _rotation_variance)))))

(fn RandomiseXYZSpacing
  (bind _spacing_variation (Variables|TOOLOPTIONS|Getspacing%20variation))
  ;[0 1 0] Random spacing based on the parameters you set in the editor
  (return (+ (Math|Random|RandomFloatinRange (- 0.0 (.x _spacing_variation)) (.x _spacing_variation)) (Variables|TOOLOPTIONS|GetX%20Spacing)) (+ (Math|Random|RandomFloatinRange (- 0.0 (.y _spacing_variation)) (.y _spacing_variation)) (Variables|TOOLOPTIONS|GetY%20spacing)) (+ (Math|Random|RandomFloatinRange (- 0.0 (.z _spacing_variation)) (.z _spacing_variation)) (Variables|TOOLOPTIONS|GetZ%20Spacing))))
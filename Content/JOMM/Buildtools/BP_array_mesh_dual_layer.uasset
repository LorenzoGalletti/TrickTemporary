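; A build tool Blueprint for JOMM that fills a configurable 3D grid with two overlapping layers of instanced static meshes.
; The construction script assigns both selected meshes, then calls a constructor event so the build shows in the editor and keeps navmesh valid in play.
; Nested X, Z and Y loops add both instances at each spaced position, skipping grid coordinates listed in Gaps for openings like doors.
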(event Custom|constructor
  ;[1 1 1] X and Z repeats (X handled as the 0 row of Z anyway)
  (for _index (range 0 (Variables|TOOLOPTIONS|GetX%20Repeats))
    (for _index_2 (range 0 (Variables|TOOLOPTIONS|GetZ%20repeats))
      ;[1 1 1] Y repeats
      (for _index_3 (range 0 (Variables|TOOLOPTIONS|GetY%20Repeats))
        (bind _continue (CallFunction|FindGaps _index _index_3 _index_2))
        (if (not _continue)
          (Components|InstancedStaticMesh|AddInstance (Variables|Default|GetH%20mesh%20to%20use) (Math|Transform|MakeTransform (Math|Vector|MakeVector (* _index (Variables|TOOLOPTIONS|GetX%20Spacing)) (* _index_3 (Variables|TOOLOPTIONS|GetY%20spacing)) (* _index_2 (Variables|TOOLOPTIONS|GetZ%20Spacing))) "0, 0, 0" "1,1,1"))
          (Components|InstancedStaticMesh|AddInstance (Variables|Default|Get2nd%20layer%20H%20mesh%20to%20use) (Math|Transform|MakeTransform (Math|Vector|MakeVector (* _index (Variables|TOOLOPTIONS|GetX%20Spacing)) (* _index_3 (Variables|TOOLOPTIONS|GetY%20spacing)) (* _index_2 (Variables|TOOLOPTIONS|GetZ%20Spacing))) "0, 0, 0" "1,1,1")))))))

(fn ConstructionScript
  ;[0 1 0] array mesh:  Mark Seddon:  JOMM (Just One More Minute)
  (Components|StaticMesh|SetStaticMesh (Variables|Default|GetH%20mesh%20to%20use) (Variables|TOOLOPTIONS|Getselect%20main%20mesh))
  (Components|StaticMesh|SetStaticMesh (Variables|Default|Get2nd%20layer%20H%20mesh%20to%20use) (Variables|TOOLOPTIONS|Getselct%202nd%20layer%20mesh))
  (CallFunction|Constructor) ; running this from here lets you see the build in editor and ensures navmesh is valid in play
)

(fn FindGaps
  (params (current%20x :type Integer) (Current%20Y :type Integer) (current%20Z :type Integer))
  ;[0 1 0] In editor you can set xyz coordinates of gaps (for doors etc)
  (return (Utilities|Array|ContainsItem (Variables|TOOLOPTIONS|GetGaps) (Math|Vector|MakeVector (Math|Conversions|ToFloat(Integer) current%20x) (Math|Conversions|ToFloat(Integer) Current%20Y) (Math|Conversions|ToFloat(Integer) current%20Z)))))
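; Construction-time builder tool that arrays a chosen static mesh in an XYZ grid as hierarchical instances, with optional lights on each instance.
; Grid coordinates listed in Gaps are skipped, leaving openings for doors and the like.
; Each instance can get a configured IES spotlight plus an optional ambient point light, placed at the mesh socket with a Z offset.
; Building in the construction script previews the layout in editor and keeps navmesh valid in play.
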(event Custom|constructor
  ;[1 1 1] X and Z repeats (X handled as the 0 row of Z anyway)
  (for _index (range 0 (Variables|TOOLOPTIONS|GetX%20Repeats))
    (for _index_2 (range 0 (Variables|TOOLOPTIONS|GetZ%20repeats))
      ;[1 1 1] Y repeats
      (for _index_3 (range 0 (Variables|TOOLOPTIONS|GetY%20Repeats))
        (bind _continue (CallFunction|FindGaps _index _index_3 _index_2))
        (if (not _continue)
          (bind _returnvalue (Components|InstancedStaticMesh|AddInstance (Variables|Default|GetH%20mesh%20to%20use) (Math|Transform|MakeTransform (Math|Vector|MakeVector (* _index (Variables|TOOLOPTIONS|GetX%20Spacing)) (* _index_3 (Variables|TOOLOPTIONS|GetY%20spacing)) (* _index_2 (Variables|TOOLOPTIONS|GetZ%20Spacing))) "0, 0, 0" "1,1,1")))
          (if (Variables|LIGHTOPTIONS|Getuse%20lights)
            (CallFunction|SpawnLight _returnvalue)))))))

(event Custom|spotlight%20details
  (bind _this_spotlight (Variables|Default|Getthis%20spotlight))
  ;[1 1 1] spotlight details
  (Rendering|Lighting|SetAttenuationRadius _this_spotlight (Variables|LIGHTOPTIONS|Getlights%20attenuation%20radius))
  (Class|LightComponent|SetIESTexture _this_spotlight (Variables|LIGHTOPTIONS|GetIES%20texture))
  (Rendering|Lighting|SetInnerConeAngle _this_spotlight (Variables|LIGHTOPTIONS|Getinner%20cone%20angle))
  (Rendering|Lighting|SetOuterConeAngle _this_spotlight (Variables|LIGHTOPTIONS|Getouter%20cone%20angle))
  (Rendering|Components|Light|SetIntensity _this_spotlight (Variables|LIGHTOPTIONS|Getlight%20intensity))
  (Class|LightComponent|SetTemperature _this_spotlight (Variables|LIGHTOPTIONS|Getlight%20temperature))
  (Rendering|Components|Light|SetCastShadows _this_spotlight (Variables|LIGHTOPTIONS|GetCasts%20shadows)))

(event Custom|spawn%20light
  (params (instance%20index :type Integer))
  (bind _z_offset (Variables|LIGHTOPTIONS|GetZ%20offset))
  (bind _h_mesh_to_use (Variables|Default|GetH%20mesh%20to%20use))
  (bind _socket_transform (Variables|Default|Getsocket%20transform))
  (bind _outinstancetransform (Components|InstancedStaticMesh|GetInstanceTransform _h_mesh_to_use instance%20index false))
  (bind _returnvalue (+ (.location _outinstancetransform) _socket_transform))
  (bind _returnvalue_2 (- (.z _returnvalue) _z_offset))
  (bind _returnvalue_3 (Math|Vector|MakeVector (.x _returnvalue) (.y _returnvalue) _returnvalue_2))
  ;[1 1 1] spawn lights with this instance
  (bind _returnvalue_4 (AddComponent|AddSpotLightComponent false (Math|Transform|MakeTransform _returnvalue_3 (Variables|LIGHTOPTIONS|Getlight%20rotation) "1,1,1")))
  (Variables|Default|Setthis%20spotlight _returnvalue_4)
  (if (Variables|LIGHTOPTIONS|Getadd%20ambient%20point%20light)
    (bind _returnvalue_5 (AddComponent|AddPointLightComponent false (Math|Transform|MakeTransform _returnvalue_3 "0, 0, 0" "1,1,1")))
    (Variables|Default|Setthis%20point%20light _returnvalue_5)
    (CallFunction|AmbientLightDetails))
  (CallFunction|SpotlightDetails))

(event Custom|ambient%20light%20details
  ;[1 1 1] ambient light if used
  (Class|LightComponent|SetTemperature (Variables|Default|Getthis%20point%20light) (Variables|LIGHTOPTIONS|Getlight%20temperature)))

(fn ConstructionScript
  ;[0 1 0] array mesh lights:  Mark Seddon:  JOMM (Just One More Minute)
  (Components|StaticMesh|SetStaticMesh (Variables|Default|GetH%20mesh%20to%20use) (Variables|TOOLOPTIONS|Getselect%20main%20mesh))
  (Variables|Default|Setsocket%20transform (.location (Transformation|GetSocketTransform (Variables|Default|GetH%20mesh%20to%20use) (Variables|LIGHTOPTIONS|Getsocket%20name) "RTS_Component"))) ; 0 if socket does not exist
  (CallFunction|Constructor) ; running this from here lets you see the build in editor and ensures navmesh is valid in play
)

(fn FindGaps
  (params (current%20x :type Integer) (Current%20Y :type Integer) (current%20Z :type Integer))
  ;[0 1 0] In editor you can set xyz coordinates of gaps (for doors etc)
  (return (Utilities|Array|ContainsItem (Variables|TOOLOPTIONS|GetGaps) (Math|Vector|MakeVector (Math|Conversions|ToFloat(Integer) current%20x) (Math|Conversions|ToFloat(Integer) Current%20Y) (Math|Conversions|ToFloat(Integer) current%20Z)))))
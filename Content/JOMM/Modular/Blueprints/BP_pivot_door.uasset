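; Proximity-triggered automatic door Blueprint, with no lock, that either slides or pivots two hinge components in opposite directions, selected by DoorType.
; Proximity begin and end overlaps check the open flag, then after a short delay a FlipFlop plays or reverses one timeline with open or close audio.
; The timeline lerps each hinge's X location or yaw toward Slidelimit or its negation.
; The construction script derives that negation and sets playback rate from Slidetime.
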(event OnComponentBeginOverlap(proximity)
  (params (OverlappedComponent :type Primitive%20Component%20Object%20Reference) (OtherActor :type Actor%20Object%20Reference) (OtherComp :type Primitive%20Component%20Object%20Reference) (OtherBodyIndex :type Integer) (bFromSweep :type Boolean) (SweepResult :type Hit%20Result%20Structure%20%28by%20ref%29))
  ;[1 1 1] automatic doors
  (if (not (Variables|DOOROPTIONS|Getisdooropen))
    (Utilities|FlowControl|Delay 0.2)
    (CallFunction|OperatetheDoor)))

(event OnComponentEndOverlap(proximity)
  (params (OverlappedComponent :type Primitive%20Component%20Object%20Reference) (OtherActor :type Actor%20Object%20Reference) (OtherComp :type Primitive%20Component%20Object%20Reference) (OtherBodyIndex :type Integer))
  ;[1 1 1] automatic doors
  (if (Variables|DOOROPTIONS|Getisdooropen)
    (Utilities|FlowControl|Delay 0.2)
    (CallFunction|OperatetheDoor)))

(event Custom|operate%20the%20door
  ;[1 1 1] open/close a door (no lock)
  (switch Utilities|FlowControl|Switch|SwitchonE_doortypes (Variables|DOOROPTIONS|Getdoor%20type)
    (:NewEnumerator0
      _)
    (:NewEnumerator1
      _))
  (CallFunction|SlidingorPivotDoors))

(event Custom|sliding%20or%20pivot%20doors
  ;[1 1 1] single  or double sliding door option
  (bind _isa (Utilities|FlowControl|FlipFlop)
    (:A
      (Variables|DOOROPTIONS|Setisdooropen true)
      (Audio|Components|Audio|Play (Variables|Default|Getaudio_open) 0.0) ; open
      (bind _lerp_position (Timeline|Timeline_0 Play)
        (:Update
          (switch Utilities|FlowControl|Switch|SwitchonE_doortypes (Variables|DOOROPTIONS|Getdoor%20type)
            (:NewEnumerator0
              (Transformation|SetRelativeLocation (Variables|Default|Gethinge) (Math|Vector|MakeVector (Math|Float|Lerp 0.0 (Variables|DOOROPTIONS|Getslidelimit) _lerp_position) 0.0 0.0) false false)
              (Transformation|SetRelativeLocation (Variables|Default|Getsecondhinge) (Math|Vector|MakeVector (Math|Float|Lerp 0.0 (Variables|Default|Getseconddoor) _lerp_position) 0.0 0.0) false false))
            (:NewEnumerator1
              (Transformation|SetRelativeRotation (Variables|Default|Gethinge) (Math|Rotator|MakeRotator 0.0 0.0 (Math|Float|Lerp 0.0 (Variables|DOOROPTIONS|Getslidelimit) _lerp_position)) false false)
              (Transformation|SetRelativeRotation (Variables|Default|Getsecondhinge) (Math|Rotator|MakeRotator 0.0 0.0 (Math|Float|Lerp 0.0 (Variables|Default|Getseconddoor) _lerp_position)) false false))))
        (:Finished
          (Variables|DOOROPTIONS|Setisdooropen _isa))))
    (:B
      (Audio|Components|Audio|Play (Variables|Default|Getaudio_close) 0.0)
      (Timeline|Timeline_0 Reverse))))

(fn ConstructionScript
  (Variables|Default|Setseconddoor (- 0.0 (Variables|DOOROPTIONS|Getslidelimit)))
  (Components|Timeline|SetPlayRate (Variables|Default|GetTimeline_0) (/ 1.0 (Variables|DOOROPTIONS|Getslidetime))))
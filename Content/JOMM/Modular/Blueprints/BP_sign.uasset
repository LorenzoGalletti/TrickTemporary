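; BP_sign is a modular signpost actor with editable text and trim colour.
; Its construction script writes SignpostText to a text render component and creates a dynamic instance of the M_emmissive material on the mesh's second slot.
; TrimColour drives both that material's colour parameter and the text colour, so the sign updates at edit time with no active runtime logic.
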(event Collision|EventActorBeginOverlap
  (params (OtherActor :type Actor%20Object%20Reference)))

(event EventTick
  (params (DeltaSeconds :type Float%20%28single-precision%29)))

(fn ConstructionScript
  (Rendering|Components|TextRender|SetText (Variables|Default|GetTextRender) (Variables|Signoptions|Getsignpost%20text))
  (bind _returnvalue (Rendering|Material|CreateDynamicMaterialInstance (Variables|Default|GetStaticMesh) 1 "/Game/JOMM/Materials/M_emmissive.M_emmissive" "None" :!class /Script/Engine.PrimitiveComponent))
  (bind _output_get (Variables|Default|Setmat_inst1 _returnvalue))
  (Rendering|Material|SetVectorParameterValue _output_get "colour" (Variables|SignOptions|Gettrim_colour) :!class /Script/Engine.MaterialInstanceDynamic)
  (Rendering|Components|TextRender|SetTextRenderColor (Variables|Default|GetTextRender) (Math|Conversions|ToColor(LinearColor) (Variables|SignOptions|Gettrim_colour))))